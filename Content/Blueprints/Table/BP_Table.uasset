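; Puzzle table with three rotatable statues that spawns a BP_Nota_M2 note at a fixed location once all three are activated.
; Each statue's player sphere enables input and opens a gate, so RotateInteract plays a timeline turning it 90 degrees in yaw.
; Detection boxes overlapping ActivadorPuzzle-tagged actors set each activation flag and show its Niagara effect.
; A looping one-second timer checks the flags, with DoOnce limiting the spawn.
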(event OnComponentBeginOverlap(BoxDetection4)
  (params (OverlappedComponent :type Primitive%20Component%20Object%20Reference) (OtherActor :type Actor%20Object%20Reference) (OtherComp :type Primitive%20Component%20Object%20Reference) (OtherBodyIndex :type Integer) (bFromSweep :type Boolean) (SweepResult :type Hit%20Result%20Structure%20%28by%20ref%29))
  ;[1 1 1] Detector B
  (if (Actor|ActorHasTag OtherActor "ActivadorPuzzle")
    (Variables|Default|SetStatue2Activada true)
    (Development|SetHiddeninGame (Variables|Default|GetNiagaraB) false false)))

(event OnComponentBeginOverlap(SpherePlayer)
  (params (OverlappedComponent :type Primitive%20Component%20Object%20Reference) (OtherActor :type Actor%20Object%20Reference) (OtherComp :type Primitive%20Component%20Object%20Reference) (OtherBodyIndex :type Integer) (bFromSweep :type Boolean) (SweepResult :type Hit%20Result%20Structure%20%28by%20ref%29))
  ;[1 1 1] Statue 1
  (if (Actor|ActorHasTag OtherActor "Player0")
    (Input|EnableInput (Game|GetPlayerController 0))
    (Utilities|FlowControl|Gate true) ; enters at Open
  ))

(event OnComponentEndOverlap(SpherePlayer)
  (params (OverlappedComponent :type Primitive%20Component%20Object%20Reference) (OtherActor :type Actor%20Object%20Reference) (OtherComp :type Primitive%20Component%20Object%20Reference) (OtherBodyIndex :type Integer))
  ;[1 1 1] Statue 1
  (if (Actor|ActorHasTag OtherActor "Player0")
    (Input|DisableInput (Game|GetPlayerController 0))
    (Utilities|FlowControl|Gate true) ; enters at Close
  ))

(event OnComponentBeginOverlap(SpherePlayer2)
  (params (OverlappedComponent :type Primitive%20Component%20Object%20Reference) (OtherActor :type Actor%20Object%20Reference) (OtherComp :type Primitive%20Component%20Object%20Reference) (OtherBodyIndex :type Integer) (bFromSweep :type Boolean) (SweepResult :type Hit%20Result%20Structure%20%28by%20ref%29))
  ;[1 1 1] Statue 2
  (if (Actor|ActorHasTag OtherActor "Player0")
    (Input|EnableInput (Game|GetPlayerController 0))
    (Utilities|FlowControl|Gate true) ; enters at Open
  ))

(event OnComponentEndOverlap(SpherePlayer2)
  (params (OverlappedComponent :type Primitive%20Component%20Object%20Reference) (OtherActor :type Actor%20Object%20Reference) (OtherComp :type Primitive%20Component%20Object%20Reference) (OtherBodyIndex :type Integer))
  ;[1 1 1] Statue 2
  (if (Actor|ActorHasTag OtherActor "Player0")
    (Input|DisableInput (Game|GetPlayerController 0))
    (Utilities|FlowControl|Gate true) ; enters at Close
  ))

(event OnComponentBeginOverlap(SpherePlayer3)
  (params (OverlappedComponent :type Primitive%20Component%20Object%20Reference) (OtherActor :type Actor%20Object%20Reference) (OtherComp :type Primitive%20Component%20Object%20Reference) (OtherBodyIndex :type Integer) (bFromSweep :type Boolean) (SweepResult :type Hit%20Result%20Structure%20%28by%20ref%29))
  ;[1 1 1] Statue 3
  (if (Actor|ActorHasTag OtherActor "Player0")
    (Input|EnableInput (Game|GetPlayerController 0))
    (Utilities|FlowControl|Gate true) ; enters at Open
  ))

(event OnComponentEndOverlap(SpherePlayer3)
  (params (OverlappedComponent :type Primitive%20Component%20Object%20Reference) (OtherActor :type Actor%20Object%20Reference) (OtherComp :type Primitive%20Component%20Object%20Reference) (OtherBodyIndex :type Integer))
  ;[1 1 1] Statue 3
  (if (Actor|ActorHasTag OtherActor "Player0")
    (Input|DisableInput (Game|GetPlayerController 0))
    (Utilities|FlowControl|Gate true) ; enters at Close
  ))

(event OnComponentEndOverlap(BoxDetection4)
  (params (OverlappedComponent :type Primitive%20Component%20Object%20Reference) (OtherActor :type Actor%20Object%20Reference) (OtherComp :type Primitive%20Component%20Object%20Reference) (OtherBodyIndex :type Integer))
  ;[1 1 1] Detector B
  (if (Actor|ActorHasTag OtherActor "ActivadorPuzzle")
    (Variables|Default|SetStatue2Activada false)
    (Development|SetHiddeninGame (Variables|Default|GetNiagaraB) true false)))

(event OnComponentBeginOverlap(BoxDetection5)
  (params (OverlappedComponent :type Primitive%20Component%20Object%20Reference) (OtherActor :type Actor%20Object%20Reference) (OtherComp :type Primitive%20Component%20Object%20Reference) (OtherBodyIndex :type Integer) (bFromSweep :type Boolean) (SweepResult :type Hit%20Result%20Structure%20%28by%20ref%29))
  ;[1 1 1] Detector C
  (if (Actor|ActorHasTag OtherActor "ActivadorPuzzle")
    (Variables|Default|SetStatue3Activada true)
    (Development|SetHiddeninGame (Variables|Default|GetNiagaraC) false false)))

(event OnComponentEndOverlap(BoxDetection5)
  (params (OverlappedComponent :type Primitive%20Component%20Object%20Reference) (OtherActor :type Actor%20Object%20Reference) (OtherComp :type Primitive%20Component%20Object%20Reference) (OtherBodyIndex :type Integer))
  ;[1 1 1] Detector C
  (if (Actor|ActorHasTag OtherActor "ActivadorPuzzle")
    (Variables|Default|SetStatue3Activada false)
    (Development|SetHiddeninGame (Variables|Default|GetNiagaraC) true false)))

(event OnComponentBeginOverlap(BoxDetection)
  (params (OverlappedComponent :type Primitive%20Component%20Object%20Reference) (OtherActor :type Actor%20Object%20Reference) (OtherComp :type Primitive%20Component%20Object%20Reference) (OtherBodyIndex :type Integer) (bFromSweep :type Boolean) (SweepResult :type Hit%20Result%20Structure%20%28by%20ref%29))
  ;[1 1 1] Activador A
  (if (Actor|ActorHasTag OtherActor "ActivadorPuzzle")
    (Variables|Default|SetStatue1Activada true)
    (Development|SetHiddeninGame (Variables|Default|GetNiagaraA) false false)))

(event OnComponentEndOverlap(BoxDetection)
  (params (OverlappedComponent :type Primitive%20Component%20Object%20Reference) (OtherActor :type Actor%20Object%20Reference) (OtherComp :type Primitive%20Component%20Object%20Reference) (OtherBodyIndex :type Integer))
  ;[1 1 1] Activador A
  (if (Actor|ActorHasTag OtherActor "ActivadorPuzzle")
    (Variables|Default|SetStatue1Activada false)
    (Development|SetHiddeninGame (Variables|Default|GetNiagaraA) true false)))

(event Custom|PuzzleResulto
  (if (Math|Boolean|ANDBoolean (Variables|Default|GetStatue1Activada) (Variables|Default|GetStatue2Activada) (Variables|Default|GetStatue3Activada))
    (Utilities|FlowControl|DoOnce false
      (:Completed
        (Game|SpawnActorfromClass "/Game/Blueprints/Notes/BP_Nota_M2.BP_Nota_M2_C" (Math|Transform|MakeTransform "669.000000,-1090.000000,706.000000" "0, 0, 0" "1.000000,1.000000,1.000000") "Undefined" "MultiplyWithRoot" 0 0)))))

(event EventBeginPlay
  (Utilities|Time|SetTimerbyEvent (delegate Custom|PuzzleResulto) 1.0 true)
  (Variables|StatuesRotations|SetWorldRotationStatueA (Transformation|GetWorldRotation (Variables|Default|GetSatanA)))
  (Variables|StatuesRotations|SetWorldRotationStatueB (Transformation|GetWorldRotation (Variables|Default|GetSatanB)))
  (Variables|StatuesRotations|SetWorldRotationStatueC (Transformation|GetWorldRotation (Variables|Default|GetSatanC))))

(event Input|ActionEvents|InputActionRotateInteract
  (params (Key :type Key%20Structure :default "None"))
  ;[1 1 1] Statue 3
  (:Pressed
    (Utilities|FlowControl|Gate true
      (:Exit
        (Input|DisableInput (Game|GetPlayerController 0))
        (bind _newtrack_0 (Timeline|Timeline3 PlayFromStart)
          (:Update
            (Transformation|SetRelativeRotation (Variables|Default|GetSatanC) (Math|Rotator|Lerp(Rotator) (Variables|StatuesRotations|GetWorldRotationStatueC) (Math|Rotator|MakeRotator (.Roll (Math|Rotator|BreakRotator (Variables|StatuesRotations|GetWorldRotationStatueC))) (.Pitch (Math|Rotator|BreakRotator (Variables|StatuesRotations|GetWorldRotationStatueC))) (+ (.Yaw (Math|Rotator|BreakRotator (Variables|StatuesRotations|GetWorldRotationStatueC))) 9e+01)) _newtrack_0) false false))
          (:Finished
            (Variables|StatuesRotations|SetWorldRotationStatueC (Math|Rotator|Lerp(Rotator) (Variables|StatuesRotations|GetWorldRotationStatueC) (Math|Rotator|MakeRotator (.Roll (Math|Rotator|BreakRotator (Variables|StatuesRotations|GetWorldRotationStatueC))) (.Pitch (Math|Rotator|BreakRotator (Variables|StatuesRotations|GetWorldRotationStatueC))) (+ (.Yaw (Math|Rotator|BreakRotator (Variables|StatuesRotations|GetWorldRotationStatueC))) 9e+01)) _newtrack_0))
            (Input|EnableInput (Game|GetPlayerController 0))))))))

(event Input|ActionEvents|InputActionRotateInteract
  (params (Key :type Key%20Structure :default "None"))
  ;[1 1 1] Statue 1
  (:Pressed
    (Utilities|FlowControl|Gate true
      (:Exit
        (Input|DisableInput (Game|GetPlayerController 0))
        (bind _newtrack_0 (Timeline|TimelineStatue PlayFromStart)
          (:Update
            (Transformation|SetRelativeRotation (Variables|Default|GetSatanA) (Math|Rotator|Lerp(Rotator) (Variables|StatuesRotations|GetWorldRotationStatueA) (Math|Rotator|MakeRotator (.Roll (Math|Rotator|BreakRotator (Variables|StatuesRotations|GetWorldRotationStatueA))) (.Pitch (Math|Rotator|BreakRotator (Variables|StatuesRotations|GetWorldRotationStatueA))) (+ (.Yaw (Math|Rotator|BreakRotator (Variables|StatuesRotations|GetWorldRotationStatueA))) 9e+01)) _newtrack_0) false false))
          (:Finished
            (Variables|StatuesRotations|SetWorldRotationStatueA (Math|Rotator|Lerp(Rotator) (Variables|StatuesRotations|GetWorldRotationStatueA) (Math|Rotator|MakeRotator (.Roll (Math|Rotator|BreakRotator (Variables|StatuesRotations|GetWorldRotationStatueA))) (.Pitch (Math|Rotator|BreakRotator (Variables|StatuesRotations|GetWorldRotationStatueA))) (+ (.Yaw (Math|Rotator|BreakRotator (Variables|StatuesRotations|GetWorldRotationStatueA))) 9e+01)) _newtrack_0))
            (Input|EnableInput (Game|GetPlayerController 0))))))))

(event Input|ActionEvents|InputActionRotateInteract
  (params (Key :type Key%20Structure :default "None"))
  ;[1 1 1] Statue 2
  (:Pressed
    (Utilities|FlowControl|Gate true
      (:Exit
        (Input|DisableInput (Game|GetPlayerController 0))
        (bind _newtrack_0 (Timeline|Timeline2 PlayFromStart)
          (:Update
            (Transformation|SetRelativeRotation (Variables|Default|GetSatanB) (Math|Rotator|Lerp(Rotator) (Variables|StatuesRotations|GetWorldRotationStatueB) (Math|Rotator|MakeRotator (.Roll (Math|Rotator|BreakRotator (Variables|StatuesRotations|GetWorldRotationStatueB))) (.Pitch (Math|Rotator|BreakRotator (Variables|StatuesRotations|GetWorldRotationStatueB))) (+ (.Yaw (Math|Rotator|BreakRotator (Variables|StatuesRotations|GetWorldRotationStatueB))) 9e+01)) _newtrack_0) false false))
          (:Finished
            (Variables|StatuesRotations|SetWorldRotationStatueB (Math|Rotator|Lerp(Rotator) (Variables|StatuesRotations|GetWorldRotationStatueB) (Math|Rotator|MakeRotator (.Roll (Math|Rotator|BreakRotator (Variables|StatuesRotations|GetWorldRotationStatueB))) (.Pitch (Math|Rotator|BreakRotator (Variables|StatuesRotations|GetWorldRotationStatueB))) (+ (.Yaw (Math|Rotator|BreakRotator (Variables|StatuesRotations|GetWorldRotationStatueB))) 9e+01)) _newtrack_0))
            (Input|EnableInput (Game|GetPlayerController 0))))))))

(fn ConstructionScript)

(fn IsOneInteract?
  (return false))