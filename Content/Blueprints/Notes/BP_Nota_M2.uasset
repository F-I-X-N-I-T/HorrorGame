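; BP_Nota_M2 is an interactable note pickup that, on Interact, calls SumaA on the BP_ThirdPersonCharacter and destroys itself.
; SpawnWidget shows supplied text in WBP_Notes while blocking move and look input, and CloseWidget restores input, removes the widget and destroys the actor.
; Interact calls neither widget function, and the PickUpNoteMessage call is disconnected.
; IsOneInteract always returns false.
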(event EventInteract
  (bind _returnvalue (Actor|GetActorOfClass "/Game/ThirdPerson/Blueprints/BP_ThirdPersonCharacter.BP_ThirdPersonCharacter_C"))
  (Default|SumaA _returnvalue)
  (Actor|DestroyActor))

(fn ConstructionScript)

(fn SpawnWidget
  (params (InText :type Text))
  (bind _returnvalue (Game|GetPlayerController 0))
  (Input|SetIgnoreMoveInput _returnvalue true)
  (Input|SetIgnoreLookInput _returnvalue true)
  (bind _returnvalue_2 (UserInterface|CreateWidget "/Game/Blueprints/UI/Notes/WBP_Notes.WBP_Notes_C" (Game|GetPlayerController 0)))
  (Variables|Default|SetWBP%20Notes _returnvalue_2)
  (Rendering|Components|TextRender|SetText (Variables|/Game/Blueprints/UI/Notes/WBP_Notes.WBP_Notes_C|GetNotaText (Variables|Default|GetWBP%20Notes)) InText)
  (UserInterface|Viewport|AddtoViewport (Variables|Default|GetWBP%20Notes) 0))

(fn CloseWidget
  (bind _returnvalue (Game|GetPlayerController 0))
  (Input|SetIgnoreMoveInput _returnvalue false)
  (Input|SetIgnoreLookInput _returnvalue false)
  (Widget|RemovefromParent (Variables|Default|GetWBP%20Notes))
  (Actor|DestroyActor))

(fn IsOneInteract?
  (return false))