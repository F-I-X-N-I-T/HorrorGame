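; Password-locked door that opens only with the correct code and once the player character has collected seven notes.
; Interact spawns a keypad widget, freezing move and look input, and binds its buttons to build, clear, cancel or submit the typed code.
; A successful submit sets PasswordIsEqual and calls InteractDoorPassword, so later interactions skip the keypad.
; A wrong code just closes the widget; missing notes also print a warning and reset the unlock flag.
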(event Custom|OnClicked_Event6
  (bind _output_get (Variables|Widget|SetInput (Utilities|String|Append (Variables|Widget|GetInput) "5")))
  (Rendering|Components|TextRender|SetText (Variables|/Game/Blueprints/UI/Doors/WBP_DoorPassword.WBP_DoorPassword_C|GetText_Code (Variables|Widget|GetWBP_DoorPassword)) (Utilities|Text|ToText(String) _output_get)))

(event Custom|OnClicked_Event7
  (bind _output_get (Variables|Widget|SetInput (Utilities|String|Append (Variables|Widget|GetInput) "6")))
  (Rendering|Components|TextRender|SetText (Variables|/Game/Blueprints/UI/Doors/WBP_DoorPassword.WBP_DoorPassword_C|GetText_Code (Variables|Widget|GetWBP_DoorPassword)) (Utilities|Text|ToText(String) _output_get)))

(event Custom|OnClicked_Event8
  (bind _output_get (Variables|Widget|SetInput (Utilities|String|Append (Variables|Widget|GetInput) "7")))
  (Rendering|Components|TextRender|SetText (Variables|/Game/Blueprints/UI/Doors/WBP_DoorPassword.WBP_DoorPassword_C|GetText_Code (Variables|Widget|GetWBP_DoorPassword)) (Utilities|Text|ToText(String) _output_get)))

(event Custom|OnClicked_Event9
  (bind _output_get (Variables|Widget|SetInput (Utilities|String|Append (Variables|Widget|GetInput) "8")))
  (Rendering|Components|TextRender|SetText (Variables|/Game/Blueprints/UI/Doors/WBP_DoorPassword.WBP_DoorPassword_C|GetText_Code (Variables|Widget|GetWBP_DoorPassword)) (Utilities|Text|ToText(String) _output_get)))

(event Custom|OnClicked_Event10
  (bind _output_get (Variables|Widget|SetInput (Utilities|String|Append (Variables|Widget|GetInput) "9")))
  (Rendering|Components|TextRender|SetText (Variables|/Game/Blueprints/UI/Doors/WBP_DoorPassword.WBP_DoorPassword_C|GetText_Code (Variables|Widget|GetWBP_DoorPassword)) (Utilities|Text|ToText(String) _output_get)))

(event Custom|OnClicked_Event11
  (bind _output_get (Variables|Widget|SetInput (Utilities|String|Append (Variables|Widget|GetInput) "0")))
  (Rendering|Components|TextRender|SetText (Variables|/Game/Blueprints/UI/Doors/WBP_DoorPassword.WBP_DoorPassword_C|GetText_Code (Variables|Widget|GetWBP_DoorPassword)) (Utilities|Text|ToText(String) _output_get)))

(event Custom|OnClicked_Event12
  (bind _output_get (Variables|Widget|SetInput ""))
  (Rendering|Components|TextRender|SetText (Variables|/Game/Blueprints/UI/Doors/WBP_DoorPassword.WBP_DoorPassword_C|GetText_Code (Variables|Widget|GetWBP_DoorPassword)) (Utilities|Text|ToText(String) _output_get)))

(event Custom|OnClicked_Event13
  ;[1 1 1] la pss es correcta? -si abre la puerta
  (if (Utilities|Enum|Equal(Enum) (Variables|Widget|GetInput) (Variables|Widget|GetPassword))
    (Variables|Widget|SetPasswordIsEqual true)
    (bind _returnvalue (Actor|GetActorOfClass "/Game/ThirdPerson/Blueprints/BP_ThirdPersonCharacter.BP_ThirdPersonCharacter_C"))
    ;[1 1 1] Tiene todas las notas?-si abre la puerta. No- le pide que necesita las notas
    (if (== (Variables|/Game/ThirdPerson/Blueprints/BP_ThirdPersonCharacter.BP_ThirdPersonCharacter_C|GetSumNotes _returnvalue) 7)
      (Class|DoorPassword|InteractDoorPassword false)
      (Variables|Widget|SetPasswordIsEqual true)
      ;[1 1 1] Desbloquea la puerta
      (CallFunction|CloseWidget)
      (else
        (Development|PrintString "Necesitas todas las notas")
        (Variables|Widget|SetPasswordIsEqual false)
        (Variables|Widget|SetInput "")
        (CallFunction|CloseWidget)))
    (else
      (CallFunction|CloseWidget)
      (Variables|Widget|SetInput ""))))

(event Custom|OnClicked_Event
  ;[1 1 1] Cierra el widget y limpia la var input del widget
  (CallFunction|CloseWidget)
  (Variables|Widget|SetInput ""))

(event Custom|OnClicked_Event2
  (bind _output_get (Variables|Widget|SetInput (Utilities|String|Append (Variables|Widget|GetInput) "1")))
  (Rendering|Components|TextRender|SetText (Variables|/Game/Blueprints/UI/Doors/WBP_DoorPassword.WBP_DoorPassword_C|GetText_Code (Variables|Widget|GetWBP_DoorPassword)) (Utilities|Text|ToText(String) _output_get)))

(event Custom|OnClicked_Event3
  (bind _output_get (Variables|Widget|SetInput (Utilities|String|Append (Variables|Widget|GetInput) "2")))
  (Rendering|Components|TextRender|SetText (Variables|/Game/Blueprints/UI/Doors/WBP_DoorPassword.WBP_DoorPassword_C|GetText_Code (Variables|Widget|GetWBP_DoorPassword)) (Utilities|Text|ToText(String) _output_get)))

(event Custom|OnClicked_Event4
  (bind _output_get (Variables|Widget|SetInput (Utilities|String|Append (Variables|Widget|GetInput) "3")))
  (Rendering|Components|TextRender|SetText (Variables|/Game/Blueprints/UI/Doors/WBP_DoorPassword.WBP_DoorPassword_C|GetText_Code (Variables|Widget|GetWBP_DoorPassword)) (Utilities|Text|ToText(String) _output_get)))

(event Custom|OnClicked_Event5
  (bind _output_get (Variables|Widget|SetInput (Utilities|String|Append (Variables|Widget|GetInput) "4")))
  (Rendering|Components|TextRender|SetText (Variables|/Game/Blueprints/UI/Doors/WBP_DoorPassword.WBP_DoorPassword_C|GetText_Code (Variables|Widget|GetWBP_DoorPassword)) (Utilities|Text|ToText(String) _output_get)))

(event EventInteract
  (Utilities|FlowControl|Sequence
    (:then_0
      (if (Variables|Widget|GetPasswordIsEqual)
        (Class|DoorPassword|InteractDoorPassword false)
        (else
          (CallFunction|SpawnWidget)
          ;[1 1 1] Cierra el widget y limpia la var input del widget
          (EventDispatchers|AssignOnClicked (Variables|/Game/Blueprints/UI/Doors/WBP_DoorPassword.WBP_DoorPassword_C|GetButton_Exit (Variables|Widget|GetWBP_DoorPassword)) (delegate Custom|OnClicked_Event)))))
    (:then_1
      (EventDispatchers|BindEventtoOnClicked (Variables|/Game/Blueprints/UI/Doors/WBP_DoorPassword.WBP_DoorPassword_C|GetButton_0 (Variables|Widget|GetWBP_DoorPassword)) (delegate Custom|OnClicked_Event2)))
    (:then_2
      (EventDispatchers|AssignOnClicked (Variables|/Game/Blueprints/UI/Doors/WBP_DoorPassword.WBP_DoorPassword_C|GetButton_1 (Variables|Widget|GetWBP_DoorPassword)) (delegate Custom|OnClicked_Event3)))
    (:then_3
      (EventDispatchers|AssignOnClicked (Variables|/Game/Blueprints/UI/Doors/WBP_DoorPassword.WBP_DoorPassword_C|GetButton_2 (Variables|Widget|GetWBP_DoorPassword)) (delegate Custom|OnClicked_Event4)))
    (:then_4
      (EventDispatchers|AssignOnClicked (Variables|/Game/Blueprints/UI/Doors/WBP_DoorPassword.WBP_DoorPassword_C|GetButton_3 (Variables|Widget|GetWBP_DoorPassword)) (delegate Custom|OnClicked_Event5)))
    (:then_5
      (EventDispatchers|AssignOnClicked (Variables|/Game/Blueprints/UI/Doors/WBP_DoorPassword.WBP_DoorPassword_C|GetButton_4 (Variables|Widget|GetWBP_DoorPassword)) (delegate Custom|OnClicked_Event6)))
    (:then_6
      (EventDispatchers|AssignOnClicked (Variables|/Game/Blueprints/UI/Doors/WBP_DoorPassword.WBP_DoorPassword_C|GetButton_5 (Variables|Widget|GetWBP_DoorPassword)) (delegate Custom|OnClicked_Event7)))
    (:then_7
      (EventDispatchers|AssignOnClicked (Variables|/Game/Blueprints/UI/Doors/WBP_DoorPassword.WBP_DoorPassword_C|GetButton_6 (Variables|Widget|GetWBP_DoorPassword)) (delegate Custom|OnClicked_Event8)))
    (:then_8
      (EventDispatchers|AssignOnClicked (Variables|/Game/Blueprints/UI/Doors/WBP_DoorPassword.WBP_DoorPassword_C|GetButton_7 (Variables|Widget|GetWBP_DoorPassword)) (delegate Custom|OnClicked_Event9)))
    (:then_9
      (EventDispatchers|AssignOnClicked (Variables|/Game/Blueprints/UI/Doors/WBP_DoorPassword.WBP_DoorPassword_C|GetButton_8 (Variables|Widget|GetWBP_DoorPassword)) (delegate Custom|OnClicked_Event10)))
    (:then_10
      (EventDispatchers|AssignOnClicked (Variables|/Game/Blueprints/UI/Doors/WBP_DoorPassword.WBP_DoorPassword_C|GetButton_10 (Variables|Widget|GetWBP_DoorPassword)) (delegate Custom|OnClicked_Event11)))
    (:then_11
      (EventDispatchers|AssignOnClicked (Variables|/Game/Blueprints/UI/Doors/WBP_DoorPassword.WBP_DoorPassword_C|GetButton_9 (Variables|Widget|GetWBP_DoorPassword)) (delegate Custom|OnClicked_Event12)))
    (:then_12
      (EventDispatchers|AssignOnClicked (Variables|/Game/Blueprints/UI/Doors/WBP_DoorPassword.WBP_DoorPassword_C|GetButton_11 (Variables|Widget|GetWBP_DoorPassword)) (delegate Custom|OnClicked_Event13)))))

(fn ConstructionScript)

(fn SpawnWidget
  (bind _returnvalue (Game|GetPlayerController 0))
  (bind _returnvalue_2 (Game|GetPlayerController 0))
  (Input|SetIgnoreMoveInput _returnvalue true)
  (Input|SetIgnoreLookInput _returnvalue true)
  (bind _returnvalue_3 (UserInterface|CreateWidget "/Game/Blueprints/UI/Doors/WBP_DoorPassword.WBP_DoorPassword_C" (Game|GetPlayerController 0)))
  (Variables|Widget|SetWBP_DoorPassword _returnvalue_3)
  (UserInterface|Viewport|AddtoViewport (Variables|Widget|GetWBP_DoorPassword) 0)
  (Input|SetInputModeGameandUI _returnvalue_2 (Variables|Widget|GetWBP_DoorPassword) "DoNotLock" true false)
  (Variables|/Script/Engine.PlayerController|SetbShowMouseCursor _returnvalue_2 true))

(fn CloseWidget
  (bind _returnvalue (Game|GetPlayerController 0))
  (bind _returnvalue_2 (Game|GetPlayerController 0))
  (Input|SetIgnoreMoveInput _returnvalue false)
  (Input|SetIgnoreLookInput _returnvalue false)
  (Widget|RemovefromParent (Variables|Widget|GetWBP_DoorPassword))
  (Input|SetInputModeGameOnly _returnvalue_2 false)
  (Variables|/Script/Engine.PlayerController|SetbShowMouseCursor _returnvalue_2 false))

(fn IsOneInteract?
  (return false))