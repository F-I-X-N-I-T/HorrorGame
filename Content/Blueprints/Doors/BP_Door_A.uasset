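; BP_Door_A is an interactable door that opens only after a key pickup event sets it openable, then shuts behind the player.
; Interact alternates a timeline forward and in reverse to swing the mesh yaw through 90 degrees, playing the opening sound only once.
; The first Player0 overlap with the trigger box clears the open flag, reverses the timeline and activates knocking and closing audio.
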(event OnComponentBeginOverlap(Box)
  (params (OverlappedComponent :type Primitive%20Component%20Object%20Reference) (OtherActor :type Actor%20Object%20Reference) (OtherComp :type Primitive%20Component%20Object%20Reference) (OtherBodyIndex :type Integer) (bFromSweep :type Boolean) (SweepResult :type Hit%20Result%20Structure%20%28by%20ref%29))
  ;[1 1 1] Cierra la puerta una vez el player este dentro
  (if (Actor|ActorHasTag OtherActor "Player0")
    (Utilities|FlowControl|DoOnce false
      (:Completed
        (Variables|Door|SetDoorOpen? false)
        (CallFunction|CloseDoor)
        (Components|Activation|Activate (Variables|Default|GetAudioTockTock) false)
        (Components|Activation|Activate (Variables|Default|GetAudioClose) false)))))

(event Custom|CloseDoor
  (bind _newtrack_0 (Timeline|DoorOpenAnim Reverse)
    (:Update
      (Transformation|SetRelativeRotation (Variables|Default|GetSM_Door_Outside_A4) (Math|Rotator|MakeRotator 0.0 0.0 (Math|Float|Lerp 0.0 9e+01 _newtrack_0)) false false)
      (Utilities|FlowControl|DoOnce false
        (:Completed
          (Components|Activation|Activate (Variables|Default|GetAudioOpen) false))))))

(event EventIPickUpKey
  (Variables|Door|SetDoorOpen? true))

(event EventInteract
  (if (Variables|Door|GetDoorOpen?)
    (Utilities|FlowControl|FlipFlop
      (:A
        (bind _newtrack_0 (Timeline|DoorOpenAnim PlayFromStart)
          (:Update
            (Transformation|SetRelativeRotation (Variables|Default|GetSM_Door_Outside_A4) (Math|Rotator|MakeRotator 0.0 0.0 (Math|Float|Lerp 0.0 9e+01 _newtrack_0)) false false)
            (Utilities|FlowControl|DoOnce false
              (:Completed
                (Components|Activation|Activate (Variables|Default|GetAudioOpen) false))))))
      (:B
        (Timeline|DoorOpenAnim Reverse)))))

(fn ConstructionScript)

(fn IsOneInteract?
  (return false))